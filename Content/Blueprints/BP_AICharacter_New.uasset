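; Team-based AI character Blueprint that shows team, squad-leader status and equipped weapon visually.
; Every Tick polls IsLeader and GetTeam to set a blue or red mesh overlay material, with separate leader variants.
; The leader branch casts SquadLeader and applies the outline to that character's mesh; non-leaders outline their own.
; Tick also shows only the Rifle, Pistol or Sniper component matching GetWeaponType.
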(event `self.ReceiveTick`
  (params (DeltaSeconds :type "Float (single-precision)"))
  (`self.UpdateColourByLeader`)
  (`self.SetWeaponVisibility`))

(fn `ApplyLeaderOutline`
  (params (SquadLeader :type "AICharacter Object Reference"))
  (bind _mesh (`Character.Mesh` SquadLeader))
  (bind _returnvalue (`self.GetTeam`))
  (switch `ETeam` _returnvalue
    (:`Team1`
      (`MeshComponent.SetOverlayMaterial` _mesh "/Game/Materials/BlueMaterial_Leader_Inst.BlueMaterial_Leader_Inst"))
    (:`Team2`
      (`MeshComponent.SetOverlayMaterial` _mesh "/Game/Materials/RedMaterial_Leader_Inst.RedMaterial_Leader_Inst"))))

(fn `ApplyNonLeaderOutline`
  (bind _mesh (`self.Mesh`))
  (bind _returnvalue (`self.GetTeam`))
  (switch `ETeam` _returnvalue
    (:`Team1`
      (`MeshComponent.SetOverlayMaterial` _mesh "/Game/Materials/BlueMaterial_Inst.BlueMaterial_Inst"))
    (:`Team2`
      (`MeshComponent.SetOverlayMaterial` _mesh "/Game/Materials/RedMaterial_Inst.RedMaterial_Inst"))))

(fn `SetWeaponVisibility`
  (bind _returnvalue (`self.GetWeaponType`))
  (`SceneComponent.SetVisibility` (`self.Rifle`) (`|EnumEquality` _returnvalue "Rifle") true)
  (`SceneComponent.SetVisibility` (`self.Pistol`) (`|EnumEquality` _returnvalue "Pistol") true)
  (`SceneComponent.SetVisibility` (`self.Sniper`) (`|EnumEquality` _returnvalue "Sniper") true))

(fn `UpdateColourByLeader`
  (bind _returnvalue (`self.IsLeader`))
  (if _returnvalue
    (bind _asbp_aicharacter_new (cast `/Game/Blueprints/BP_AICharacter_New` (`self.SquadLeader`)))
    (`self.ApplyLeaderOutline` _asbp_aicharacter_new)
    (else
      (`self.ApplyNonLeaderOutline`))))

(fn `UserConstructionScript`)